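; Cowboy1 arms partial character Blueprint that keeps its scene component turned toward the first player.
; Each tick, if that player character is valid, it computes a look-at rotation from the component to the player and rebuilds the world rotation from that rotation's X and Y.
; AnyDamage calls the parent event and then forwards the same data to OnReceiveAnyDamage.
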(event `self.ReceiveBeginPlay`)

(event `self.ReceiveActorBeginOverlap`
  (params (OtherActor :type "Actor Object Reference")))

(event `self.ReceiveTick`
  (params (DeltaSeconds :type "Float (single-precision)"))
  (bind _returnvalue (`GameplayStatics.GetPlayerCharacter` null))
  (bind _scenecomponent (`self.SceneComponent`))
  (bind (_x _y) (`KismetMathLibrary.BreakRotIntoAxes` (`KismetMathLibrary.FindLookAtRotation` (`SceneComponent.K2_GetComponentLocation` _scenecomponent) (`self.K2_GetActorLocation` _returnvalue))))
  (`/Engine/EditorBlueprintResources/StandardMacros.IsValid` _returnvalue
    (:`Is Valid`
      (`SceneComponent.K2_SetWorldRotation` _scenecomponent (`KismetMathLibrary.MakeRotFromXY` _x _y) false false))))

(event `self.ReceiveAnyDamage`
  (params (Damage :type "Float (single-precision)") (DamageType :type "DamageType Object Reference") (InstigatedBy :type "Controller Object Reference") (DamageCauser :type "Actor Object Reference"))
  ;[1 1 1] Redirect none-virtual required events for damage handling
  (`parent.ReceiveAnyDamage` Damage DamageType InstigatedBy DamageCauser)
  (`self.OnReceiveAnyDamage` Damage DamageType InstigatedBy DamageCauser))

(fn `UserConstructionScript`)