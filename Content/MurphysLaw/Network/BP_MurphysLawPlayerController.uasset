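; Player controller for Murphy's Law that shows the pre-match team lobby.
; After post-login it creates the lobby widget, shares it with the game instance and fills it, delaying briefly on non-authority clients.
; Refresh requests, honored only before match start, rebuild both team panels with header entries and one entry per active PlayerState in GameState's PlayerArray, sorted by team.
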(event `self.ReceiveBeginPlay`)

(event `self.ReceiveTick`
  (params (DeltaSeconds :type "Float (single-precision)")))

(event `self.OnPostLoginDone`
  (`self.Create Lobby`)
  (if (not (`self.HasAuthority`))
    (`KismetSystemLibrary.Delay` 1.5))
  (`self.Refresh Player List`))

(event `self.OnRefreshPlayerList`
  (if (not (`GameMode.HasMatchStarted` (`GameplayStatics.GetGameMode`)))
    (`self.Refresh Player List`)))

(fn `Clear Lobby`
  (bind _bp_lobby (`self.BP_Lobby`))
  (bind _teama (`/Game/MurphysLaw/Menu/BP_Lobby.TeamA` _bp_lobby))
  (bind _teamb (`/Game/MurphysLaw/Menu/BP_Lobby.TeamB` _bp_lobby))
  (`PanelWidget.ClearChildren` _teama)
  (`PanelWidget.ClearChildren` _teamb)
  (bind _returnvalue (`|CreateWidget` "/Game/MurphysLaw/Menu/BP_LobbyEntry.BP_LobbyEntry_C"))
  (`TextBlock.SetText` (`/Game/MurphysLaw/Menu/BP_LobbyEntry.TextBlock_PlayerName` _returnvalue) "Team A")
  (`PanelWidget.AddChild` _teama _returnvalue)
  (bind _returnvalue_2 (`|CreateWidget` "/Game/MurphysLaw/Menu/BP_LobbyEntry.BP_LobbyEntry_C"))
  (`TextBlock.SetText` (`/Game/MurphysLaw/Menu/BP_LobbyEntry.TextBlock_PlayerName` _returnvalue_2) "Team B")
  (`PanelWidget.AddChild` _teamb _returnvalue_2))

(fn `Create Lobby`
  (bind _returnvalue (`|CreateWidget` "/Game/MurphysLaw/Menu/BP_Lobby.BP_Lobby_C"))
  (set `self.BP_Lobby` _returnvalue)
  (`UserWidget.AddToViewport` _returnvalue 0)
  (bind _asbp_game_instance (cast `/Game/MurphysLaw/Network/BP_GameInstance` (`GameplayStatics.GetGameInstance`)))
  (set `/Game/MurphysLaw/Network/BP_GameInstance.BP_Lobby` _returnvalue _asbp_game_instance))

(fn `Refresh Player List`
  (bind _bp_lobby (`self.BP_Lobby`))
  (`self.Clear Lobby`)
  ;[1 1 1] Pour chaque entré du player array, on créé un nouveau widget qui représente une entré dans le lobby. On l'ajoute ensuite dépendamment de l'équipe dans la bonne scroll bar panel
  (for _array_element (`GameState.PlayerArray` (`GameplayStatics.GetGameState`))
    (bind _asmurphys_law_player_state (cast `MurphysLawPlayerState` _array_element))
    (if (`MurphysLawPlayerState.IsActive` _asmurphys_law_player_state)
      (bind _returnvalue (`|CreateWidget` "/Game/MurphysLaw/Menu/BP_LobbyEntry.BP_LobbyEntry_C"))
      (`TextBlock.SetText` (`/Game/MurphysLaw/Menu/BP_LobbyEntry.TextBlock_PlayerName` _returnvalue) (`KismetTextLibrary.Conv_StringToText` (`PlayerState.PlayerName` _asmurphys_law_player_state)))
      (if (== (`MurphysLawPlayerState.Team` _asmurphys_law_player_state) 0)
        (`PanelWidget.AddChild` (`/Game/MurphysLaw/Menu/BP_Lobby.TeamA` _bp_lobby) _returnvalue)
        (else
          (`PanelWidget.AddChild` (`/Game/MurphysLaw/Menu/BP_Lobby.TeamB` _bp_lobby) _returnvalue))))))

(fn `UserConstructionScript`)