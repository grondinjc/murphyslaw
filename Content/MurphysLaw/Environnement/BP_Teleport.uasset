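; BP_Teleport is an environment trigger actor that sends any pawn overlapping it to a random location in the level.
; On overlap it zeroes the pawn's movement component velocity, then teleports it to a random TeleportLocations entry with zero rotation.
; The construction script fills that array with a few hardcoded world positions, using AddUnique to avoid duplicate entries.
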(event `self.ReceiveBeginPlay`)

(event `self.ReceiveActorBeginOverlap`
  (params (OtherActor :type "Actor Object Reference"))
  (bind _teleport_locations (`self.Teleport locations`))
  (bind _aspawn (cast `Pawn` OtherActor))
  (set `MovementComponent.Velocity` (0.0 0.0 0.0) (`Pawn.GetMovementComponent` _aspawn))
  (`self.K2_TeleportTo` :`self` OtherActor :`DestLocation` (`KismetArrayLibrary.Array_Get` _teleport_locations (`KismetMathLibrary.RandomIntegerInRange` 0 (- (`KismetArrayLibrary.Array_Length` _teleport_locations) 1)))))

(fn `UserConstructionScript`
  (`KismetArrayLibrary.Array_AddUnique` (`self.Teleport locations`) (-1126.27417 2444.494141 2665.728516))
  (`KismetArrayLibrary.Array_AddUnique` (`self.Teleport locations`) (-17800.0 -6980.0 5300.0))
  (`KismetArrayLibrary.Array_AddUnique` (`self.Teleport locations`) (-1550.0 1370.0 170.0)))